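; BP_target is a moving target actor whose Cube slides back and forth along the world Y axis.
; A timeline starts on BeginPlay and each update nudges the Cube from its current Y by a Lerped offset, so movement accumulates and depends on update rate.
; When it finishes, it waits briefly, restarts and uses a FlipFlop to toggle Reverse, switching direction for the next pass.
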(event `self.ReceiveBeginPlay`
  (bind _cube (`self.Cube`))
  (bind _returnvalue (`SceneComponent.K2_GetComponentToWorld` _cube))
  (bind (_direction _newtrack_0) (`Timeline|Timeline_0` :!via `PlayFromStart` :!label _label)
    (:`Update`
      (`SceneComponent.K2_SetWorldTransform` _cube (`KismetMathLibrary.MakeTransform` (`KismetMathLibrary.MakeVector` (.x (.location _returnvalue)) (`KismetMathLibrary.Lerp` (.y (.location _returnvalue)) (select `bool` (`self.reverse?`) :`false` (+ (.y (.location _returnvalue)) 5.0) :`true` (- (.y (.location _returnvalue)) 5.0)) _newtrack_0) (.z (.location _returnvalue))) (.rotation _returnvalue) (.scale _returnvalue)) false false))
    (:`Finished`
      (`KismetSystemLibrary.Delay` 2.0)
      (`|ExecutionSequence`
        (:`then_0`
          (goto _label :!via `PlayFromStart`))
        (:`then_1`
          (`/Engine/EditorBlueprintResources/StandardMacros.FlipFlop`
            (:`A`
              (set `self.reverse?` true))
            (:`B`
              (set `self.reverse?` false))))))))

(fn `UserConstructionScript`)