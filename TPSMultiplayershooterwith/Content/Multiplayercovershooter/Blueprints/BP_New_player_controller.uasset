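; Player controller for a multiplayer shooter that owns the main HUD widget and requests player spawns.
; Escape or Backspace toggles the in-game menu, switching to UI-only input with a cursor on open.
; Spawning delegates to BP_ThirdPersonGameMode with a fixed character class and assault weapon.
; Other events create or remove the HUD and relay damage, reload, sniper scope and pickup feedback to its child widgets.
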(event `Key|Escape`
  (params (Key :type "Key Structure"))
  (bind _wbp_ingamemenu (`/Game/Multiplayercovershooter/widgets/wbp_HUD.WBP_ingameMenu` (`self.HUD`)))
  ;[1 1 1] ingame mmenu
  (:`Pressed`
    (if (`Widget.IsVisible` _wbp_ingamemenu) :!label _label
      (`Widget.SetVisibility` _wbp_ingamemenu "Hidden")
      (else
        (`Widget.SetVisibility` _wbp_ingamemenu "Visible")
        (`WidgetBlueprintLibrary.SetInputMode_UIOnlyEx` self null)
        (set `self.bShowMouseCursor` true)))))

(event `Key|BackSpace`
  (params (Key :type "Key Structure"))
  ;[1 1 1] ingame mmenu
  (:`Pressed`
    (goto _label)))

(event `Spawn the player`
  ;[1 1 1] player spawn
  (bind _asbp_third_person_game_mode (cast `/Game/Multiplayercovershooter/Blueprints/BP_ThirdPersonGameMode` (`GameplayStatics.GetGameMode`)))
  (`/Game/Multiplayercovershooter/Blueprints/BP_ThirdPersonGameMode.SpawnPlayer` _asbp_third_person_game_mode self "/Game/Multiplayercovershooter/Blueprints/BP_ThirdPersonCharacter.BP_ThirdPersonCharacter_C" "/Game/Multiplayercovershooter/Blueprints/BP_weapons/BP_assault_weapon.BP_assault_weapon_C" (`self.PlayerState`)))

(event `Show HUD`
  ;[0.1531 0.5493 1] show main hud
  (`/Engine/EditorBlueprintResources/StandardMacros.IsValid` (`self.HUD`)
    (:`Is Valid`
      _)
    (:`Is Not Valid`
      (bind _returnvalue (`|CreateWidget` "/Game/Multiplayercovershooter/widgets/wbp_HUD.WBP_HUD_C" self))
      (set `self.HUD` _returnvalue)))
  (`UserWidget.AddToViewport` (`self.HUD`) 0)
  (`WidgetBlueprintLibrary.SetInputMode_GameOnly` self))

(event `hide HUD`
  ;[1 1 1] hide hud
  (`Widget.RemoveFromParent` (`self.HUD`)))

(event `damage indicator`
  (params (Target :type "Vector Structure (by ref)"))
  (bind _hud (`self.HUD`))
  ;[1 1 1] hurt and damage indicator
  (`/Engine/EditorBlueprintResources/StandardMacros.IsValid` _hud
    (:`Is Valid`
      (`/Game/Multiplayercovershooter/widgets/WBP_Damage_widget.on damage` (`/Game/Multiplayercovershooter/widgets/wbp_HUD.Damage_widget` _hud) Target))))

(event `reload time widget`
  ;[1 1 1] reload time widget
  (`/Game/Multiplayercovershooter/widgets/WBP_reload_time.set reload time visible` (`/Game/Multiplayercovershooter/widgets/wbp_HUD.WBP_reload_time` (`self.HUD`))))

(event `reload warn widget set anjim and sound PC`
  ;[1 1 1] reload warn widget set in/visible PC
  (`/Game/Multiplayercovershooter/widgets/WBP_reload_warn.reload warn widget set anim and sound` (`/Game/Multiplayercovershooter/widgets/wbp_HUD.WBP_reload_warn` (`self.HUD`))))

(event `sniper scope on`
  (bind _hud (`self.HUD`))
  ;[1 1 1] sniper scope on
  (`/Engine/EditorBlueprintResources/StandardMacros.IsValid` _hud
    (:`Is Valid`
      (`Widget.SetVisibility` (`/Game/Multiplayercovershooter/widgets/wbp_HUD.WBP_sniper_scope` _hud) "Visible")
      (`Widget.SetVisibility` (`/Game/Multiplayercovershooter/widgets/wbp_HUD.WBP_CrossHair` (`self.HUD`)) "Hidden")
      (`self.hide  pickup UI`))))

(event `sniper scope off`
  (bind _hud (`self.HUD`))
  ;[1 1 1] sniper scope off
  (`/Engine/EditorBlueprintResources/StandardMacros.IsValid` _hud
    (:`Is Valid`
      (`Widget.SetVisibility` (`/Game/Multiplayercovershooter/widgets/wbp_HUD.WBP_sniper_scope` _hud) "Hidden")
      (`Widget.SetVisibility` (`/Game/Multiplayercovershooter/widgets/wbp_HUD.WBP_CrossHair` (`self.HUD`)) "Visible"))))

(event `show pickup UI`
  (params (InText :type Text))
  (bind _hud (`self.HUD`))
  (bind _wbp_weaponinfo (`/Game/Multiplayercovershooter/widgets/wbp_HUD.WBP_weaponInfo` _hud))
  ;[1 1 1] show pickup UI
  (`/Engine/EditorBlueprintResources/StandardMacros.IsValid` _hud
    (:`Is Valid`
      (`Widget.SetVisibility` _wbp_weaponinfo "Visible")
      (`/Game/Multiplayercovershooter/widgets/WBP_weaponInfo.set weapon name` _wbp_weaponinfo InText))))

(event `hide  pickup UI`
  (bind _hud (`self.HUD`))
  ;[1 1 1] hide  pickup UI
  (`/Engine/EditorBlueprintResources/StandardMacros.IsValid` _hud
    (:`Is Valid`
      (`Widget.SetVisibility` (`/Game/Multiplayercovershooter/widgets/wbp_HUD.WBP_weaponInfo` _hud) "Hidden"))))

(fn `UserConstructionScript`)